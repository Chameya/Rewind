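; BP_Railing is a spline-driven railing that tiles a mesh along an editable path.
; The construction script measures the mesh's X bounds and divides the spline length by it to get the segment count.
; It adds a spline mesh component per segment, taking start and end points and tangents from the spline, with tangents clamped to mesh length to follow curves.
; The event graph has no runtime logic.
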(fn `UserConstructionScript`
  (bind _spline (`self.Spline`))
  (bind _spline_2 (`self.Spline`))
  (bind (_min _max) (break `Box` (`StaticMesh.GetBoundingBox` (`self.SplineMesh`))))
  (set `self.MeshLength` (.x (- _max _min)))
  (for _index (range (+ (`KismetMathLibrary.FTrunc` (/ (`SplineComponent.GetSplineLength` (`self.Spline`)) (`self.MeshLength`))) 1))
    ;[1 1 1] Spawn mesh and calculate direction
    (bind _returnvalue (`AddComponent|NODE_AddSplineMeshComponent-0`))
    (`StaticMeshComponent.SetStaticMesh` _returnvalue (`self.SplineMesh`))
    (`SplineMeshComponent.SetForwardAxis` _returnvalue "X" true)
    (bind _returnvalue_2 (* _index (`self.MeshLength`)))
    (bind _returnvalue_3 (* (+ _index 1) (`self.MeshLength`)))
    (`SplineMeshComponent.SetStartAndEnd` _returnvalue (`SplineComponent.GetLocationAtDistanceAlongSpline` _spline _returnvalue_2 "Local") (`KismetMathLibrary.ClampVectorSize` (`SplineComponent.GetTangentAtDistanceAlongSpline` _spline _returnvalue_2 "Local") 0.0 (`self.MeshLength`)) (`SplineComponent.GetLocationAtDistanceAlongSpline` _spline_2 _returnvalue_3 "Local") (`KismetMathLibrary.ClampVectorSize` (`SplineComponent.GetTangentAtDistanceAlongSpline` _spline_2 _returnvalue_3 "Local") 0.0 (`self.MeshLength`)) true)))
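; BPC_Quest is a quest component that shows the active quest on screen.
; On BeginPlay it creates a WB_ActiveQuestWidget, adds it to the viewport and keeps it hidden.
; The SetActiveQuestText event makes the widget visible and fills its title and description text from the ActiveQuest name and description.
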(event `self.ReceiveBeginPlay`
  (bind _returnvalue (`|CreateWidget` "/Game/Aziz/Quest_System/WB_ActiveQuestWidget.WB_ActiveQuestWidget_C"))
  (bind _output_get (set `self.ActiveQuestWidget` _returnvalue))
  (`UserWidget.AddToViewport` _output_get 0)
  (`Widget.SetVisibility` (`self.ActiveQuestWidget`) "Hidden"))

(event `Set Active Quest Text`
  (bind (_name _description) (break `/Game/Aziz/Quest_System/S_Quest` (`self.ActiveQuest`)))
  (`Widget.SetVisibility` (`self.ActiveQuestWidget`) "Visible")
  (`TextBlock.SetText` (`/Game/Aziz/Quest_System/WB_ActiveQuestWidget.ActiveQuestText` (`self.ActiveQuestWidget`)) (`KismetTextLibrary.Conv_StringToText` _name))
  (`TextBlock.SetText` (`/Game/Aziz/Quest_System/WB_ActiveQuestWidget.ActiveQuestDescription` (`self.ActiveQuestWidget`)) (`KismetTextLibrary.Conv_StringToText` _description)))
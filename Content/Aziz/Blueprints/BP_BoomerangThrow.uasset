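; Thrown boomerang projectile that can fly back to the player character and be re-equipped.
; RecallBoomerang enables pickup, turns on homing toward the character's Arrow1 and starts a loop re-aiming velocity at it every 0.1 seconds.
; Overlapping Box while pickup is enabled equips the boomerang on Kyle and destroys this actor.
; Box1 overlap sets PlayerCast true before testing it false, so its recall call never fires as wired.
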(event `self.ReceiveBeginPlay`)

(event `RotateToTarget`
  (bind _projectilemovement (`self.ProjectileMovement`))
  (set `MovementComponent.Velocity` (* (`KismetMathLibrary.GetDirectionUnitVector` (`self.K2_GetActorLocation`) (`SceneComponent.K2_GetComponentLocation` (`/Game/Rewind/VezamsMap/character/BP_ThirdPersonCharacterveezam.Arrow1` (stale `Recall Boomerang` _returnvalue)))) (`MovementComponent.GetMaxSpeed` _projectilemovement)) _projectilemovement :!label _label)
  (`KismetSystemLibrary.Delay` 0.1)
  (goto _label))

(event `Recall Boomerang`
  (bind _projectilemovement (`self.ProjectileMovement`))
  (set `self.CanEquipt` true)
  ;[1 1 1] Badel hedhi ki bech tbadel em character
  (bind _returnvalue (`GameplayStatics.GetActorOfClass` "/Game/Rewind/VezamsMap/character/BP_ThirdPersonCharacterveezam.BP_ThirdPersonCharacterveezam_C"))
  (`self.RotateToTarget`)
  (set `ProjectileMovementComponent.HomingTargetComponent` (`/Game/Rewind/VezamsMap/character/BP_ThirdPersonCharacterveezam.Arrow1` _returnvalue) _projectilemovement)
  (set `ProjectileMovementComponent.bIsHomingProjectile` true _projectilemovement))

(event `self.Box.OnComponentBeginOverlap`
  (params (OverlappedComponent :type "PrimitiveComponent Object Reference") (OtherActor :type "Actor Object Reference") (OtherComp :type "PrimitiveComponent Object Reference") (OtherBodyIndex :type Integer) (bFromSweep :type Boolean) (SweepResult :type "HitResult Structure (by ref)"))
  (bind _my_player_character (`/Game/Aziz/LinearQuestSystem/CommonFunctionLibrart.Cast To Kyle` OtherActor))
  (if (`self.CanEquipt`)
    (`/Game/Rewind/VezamsMap/character/BP_ThirdPersonCharacterveezam.EquipBoomerang` _my_player_character "/Game/Aziz/boomerang-001.boomerang-001")
    (`self.K2_DestroyActor`)))

(event `self.Box1.OnComponentBeginOverlap`
  (params (OverlappedComponent :type "PrimitiveComponent Object Reference") (OtherActor :type "Actor Object Reference") (OtherComp :type "PrimitiveComponent Object Reference") (OtherBodyIndex :type Integer) (bFromSweep :type Boolean) (SweepResult :type "HitResult Structure (by ref)"))
  (`/Game/Aziz/LinearQuestSystem/CommonFunctionLibrart.Cast To Kyle` OtherActor)
  (bind _output_get (set `self.PlayerCast` true))
  (if (not _output_get)
    (`self.Recall Boomerang`)))

(fn `UserConstructionScript`)
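; BP_Alpha is a warehouse robot that idles in a looping shutdown animation until a BP_DartBoard overlaps its box.
; That overlap makes a one-shot animation call and sets a started flag.
; From then on, Tick turns the robot's yaw toward the player character with a 90-degree offset and triggers the Q1_Part4_MD dialogue once through BP_DialogueActor_Child.
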(event `self.ReceiveBeginPlay`
  (`SkeletalMeshComponent.PlayAnimation` (`self.SkeletalMesh`) "/Game/Robot/Animations/Shutdown.Shutdown" true))

(event `self.Box.OnComponentBeginOverlap`
  (params (OverlappedComponent :type "PrimitiveComponent Object Reference") (OtherActor :type "Actor Object Reference") (OtherComp :type "PrimitiveComponent Object Reference") (OtherBodyIndex :type Integer) (bFromSweep :type Boolean) (SweepResult :type "HitResult Structure (by ref)"))
  (cast `/Game/Aziz/Blueprints/BP_DartBoard` OtherActor)
  (`SkeletalMeshComponent.PlayAnimation` (`self.SkeletalMesh`) null false)
  (set `self.Started?` true))

(event `TargetLock`
  (bind (_returnvalue_roll _returnvalue_pitch) (`KismetMathLibrary.BreakRotator` (`self.K2_GetActorRotation`)))
  (bind _returnvalue (`GameplayStatics.GetActorOfClass` "/Game/Rewind/VezamsMap/character/BP_ThirdPersonCharacterveezam.BP_ThirdPersonCharacterveezam_C"))
  (bind (_returnvalue_roll_2 _returnvalue_pitch_2 _returnvalue_yaw) (`KismetMathLibrary.BreakRotator` (`KismetMathLibrary.FindLookAtRotation` (`self.K2_GetActorLocation`) (`self.K2_GetActorLocation` _returnvalue))))
  (`self.K2_SetActorRotation` (`KismetMathLibrary.MakeRotator` _returnvalue_roll _returnvalue_pitch (- _returnvalue_yaw 90.0))))

(event `StartDialogue`
  (if (not (`self.DialogueStarted?`))
    (set `self.DialogueStarted?` true)
    (bind _returnvalue (`GameplayStatics.GetActorOfClass` "/Game/Robot/BP_DialogueActor_Child.BP_DialogueActor_Child_C"))
    (`/Game/Robot/BP_DialogueActor_Child.Dialogue` _returnvalue null "/Game/Rewind/Dialogue/Quest1_part4/Q1_Part4_MD.Q1_Part4_MD")
    (set `self.DialogueStarted?` true)))

(event `self.ReceiveTick`
  (params (DeltaSeconds :type "Float (single-precision)"))
  (if (`self.Started?`)
    (`self.TargetLock`)
    (`self.StartDialogue`)))

(fn `UserConstructionScript`)
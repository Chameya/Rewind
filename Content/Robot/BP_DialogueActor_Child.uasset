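; Child dialogue actor Blueprint that starts Mountea dialogue between the player character (Kyle) and itself.
; Its Dialogue function checks for another "Interactable"-tagged actor with a dialogue participant, gated by CanExecuteCosmeticEvents.
; It then assigns the supplied graph to the NPC participant and calls StartDialogueFromPlayer on Kyle.
; Box overlap events are empty, leaving Boomerang inventory-check, spawn and input-toggle logic disconnected.
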(event `self.Box.OnComponentBeginOverlap`
  (params (OverlappedComponent :type "PrimitiveComponent Object Reference") (OtherActor :type "Actor Object Reference") (OtherComp :type "PrimitiveComponent Object Reference") (OtherBodyIndex :type Integer) (bFromSweep :type Boolean) (SweepResult :type "HitResult Structure (by ref)")))

(event `self.Box.OnComponentEndOverlap`
  (params (OverlappedComponent :type "PrimitiveComponent Object Reference") (OtherActor :type "Actor Object Reference") (OtherComp :type "PrimitiveComponent Object Reference") (OtherBodyIndex :type Integer)))

(event `Key|E`
  (params (Key :type "Key Structure")))

(fn `Dialogue`
  (params (OtherActor :type "Actor Object Reference") (`Dialogue Graph` :type "MounteaDialogueGraph Object Reference"))
  (if (`self.ActorHasTag` OtherActor "Interactable")
    (if (!= OtherActor self)
      (`/Engine/EditorBlueprintResources/StandardMacros.Can Execute Cosmetic Events`
        (:`True`
          (`/Engine/EditorBlueprintResources/StandardMacros.IsValid` (`self.GetComponentByClass` OtherActor "/Script/MounteaDialogueSystem.MounteaDialogueParticipant")
            (:`Is Valid`
              (bind _my_player_character (`/Game/Aziz/LinearQuestSystem/CommonFunctionLibrart.Cast To Kyle` (`GameplayStatics.GetPlayerCharacter` 0)))
              (`MounteaDialogueParticipantStatics.SetDialogueGraph` (`self.NPC_MounteaDialogueParticipant`) `Dialogue Graph`)
              (`/Game/Characters/Kayle/character/BP_ThirdPersonCharacterveezam.Start Dialogue from Player` _my_player_character self))))))))

(fn `UserConstructionScript`
  (`parent.UserConstructionScript`))
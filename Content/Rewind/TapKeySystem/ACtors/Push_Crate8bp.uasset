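; A pushable crate actor that starts a tap-key event on Kyle, using the K key, when the player enters its box trigger.
; Entry disables the player's movement and controller yaw, then moves the capsule onto the trigger at a fixed facing.
; PressedFunctionality nudges the cube and player by fixed offsets and plays a throw animation as the push.
; Passed destroys the trigger, and nothing here restores movement.
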(event `self.Box.OnComponentBeginOverlap`
  (params (OverlappedComponent :type "PrimitiveComponent Object Reference") (OtherActor :type "Actor Object Reference") (OtherComp :type "PrimitiveComponent Object Reference") (OtherBodyIndex :type Integer) (bFromSweep :type Boolean) (SweepResult :type "HitResult Structure (by ref)"))
  (bind _returnvalue (`GameplayStatics.GetPlayerPawn` 0))
  (bind (_returnvalue_x _returnvalue_y) (`KismetMathLibrary.BreakVector` (`SceneComponent.K2_GetComponentLocation` (`self.Box`))))
  (if (== OtherActor _returnvalue)
    (`KismetSystemLibrary.PrintString` "Player Has walked in")
    (bind _my_player_character (`/Game/Aziz/LinearQuestSystem/CommonFunctionLibrart.Cast To Kyle` _returnvalue))
    (`/Game/Rewind/VezamsMap/character/BP_ThirdPersonCharacterveezam.Create Tap Key Event` _my_player_character "K" "k" false 0.0 self)
    ;[1 1 1] Stop Player and make it face the object
    (`CharacterMovementComponent.DisableMovement` (`Character.CharacterMovement` _my_player_character))
    (set `Pawn.bUseControllerRotationYaw` false _my_player_character)
    (bind _capsulecomponent (`Character.CapsuleComponent` _my_player_character))
    (bind (_returnvalue_x_2 _returnvalue_y_2 _returnvalue_z) (`KismetMathLibrary.BreakVector` (`SceneComponent.K2_GetComponentLocation` _capsulecomponent)))
    (`KismetSystemLibrary.MoveComponentTo` _capsulecomponent (`KismetMathLibrary.MakeVector` _returnvalue_x _returnvalue_y _returnvalue_z) (struct :`Yaw` 260.0))))

(event `/Game/Rewind/TapKeySystem/ACtors/Push_Crate_Interface.Pressed Functionality`
  (bind _returnvalue (`GameplayStatics.GetPlayerPawn` 0))
  (`SceneComponent.K2_AddLocalOffset` (`self.Cube`) (0.0 -10.0 0.0) false false)
  (bind _my_player_character (`/Game/Aziz/LinearQuestSystem/CommonFunctionLibrart.Cast To Kyle` _returnvalue))
  (`self.K2_AddActorLocalOffset` _returnvalue (10.0 0.0 0.0) false false)
  (bind _mesh (`Character.Mesh` _my_player_character))
  (`SkeletalMeshComponent.PlayAnimation` _mesh "/Game/Aziz/Kayle/UsedAnimations/Animations/GoalieThrow_1__UE.GoalieThrow_1__UE" false)
  (`SkeletalMeshComponent.SetPlayRate` _mesh 1.0))

(event `/Game/Rewind/TapKeySystem/ACtors/Push_Crate_Interface.passed`
  (`ActorComponent.K2_DestroyComponent` (`self.Box`)))

(fn `UserConstructionScript`)
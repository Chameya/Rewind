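; Base friendly AI character that follows a story route while the player (Kyle) is near it.
; Kyle entering or leaving its Box switches the first AIC_FriendlyBase controller found between Wait for Player and Follow Story Route, stopping movement on exit.
; Helper functions supply spline destinations from its story route array and set walk speed by movement tier.
; An AIMoveTo chain for advancing through routes is present but unconnected.
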(event `self.Box.OnComponentBeginOverlap`
  (params (OverlappedComponent :type "PrimitiveComponent Object Reference") (OtherActor :type "Actor Object Reference") (OtherComp :type "PrimitiveComponent Object Reference") (OtherBodyIndex :type Integer) (bFromSweep :type Boolean) (SweepResult :type "HitResult Structure (by ref)"))
  (`/Game/Aziz/LinearQuestSystem/CommonFunctionLibrart.Cast To Kyle` OtherActor)
  (`KismetSystemLibrary.PrintString` "PLayer in box")
  (bind _returnvalue (`GameplayStatics.GetActorOfClass` "/Game/Rewind/Ai_Friendly/AIC_FriendlyBase.AIC_FriendlyBase_C"))
  (bind _states (`/Game/Rewind/Ai_Friendly/AIC_FriendlyBase.Get Current State` _returnvalue))
  (switch `/Game/Rewind/Ai_Friendly/Enums/Friendly_AI_States` _states
    (:`NewEnumerator2`
      (`/Game/Rewind/Ai_Friendly/AIC_FriendlyBase.SetStateAsFollow StoryRoute` _returnvalue))))

(event `self.Box.OnComponentEndOverlap`
  (params (OverlappedComponent :type "PrimitiveComponent Object Reference") (OtherActor :type "Actor Object Reference") (OtherComp :type "PrimitiveComponent Object Reference") (OtherBodyIndex :type Integer))
  (`/Game/Aziz/LinearQuestSystem/CommonFunctionLibrart.Cast To Kyle` OtherActor)
  (`KismetSystemLibrary.PrintString` "PLayer out box")
  (bind _returnvalue (`GameplayStatics.GetActorOfClass` "/Game/Rewind/Ai_Friendly/AIC_FriendlyBase.AIC_FriendlyBase_C"))
  (bind _states (`/Game/Rewind/Ai_Friendly/AIC_FriendlyBase.Get Current State` _returnvalue))
  (switch `/Game/Rewind/Ai_Friendly/Enums/Friendly_AI_States` _states
    (:`NewEnumerator1`
      (`Controller.StopMovement` _returnvalue)
      (`/Game/Rewind/Ai_Friendly/AIC_FriendlyBase.SetStateAsWaitForPlayer` _returnvalue))))

(fn `GetStoryRoute`
  (returns (`Story Route` :type "Array of /Game/Rewind/Ai_Friendly/Bp_Story_Route Object Reference"))
  (return (`self.StoryRoute`)))

(fn `MoveAlongStoryRoute`
  (params (`StoryRoute num` :type Integer))
  (returns (Location :type "Vector Structure") (Output :type "/Game/Rewind/Ai_Friendly/Bp_Story_Route Object Reference"))
  (bind _story_route (`/Game/Rewind/Ai_Enemy/AI/BPI_Interface.GetStoryRoute`))
  (bind _output (`|GetArrayItem` _story_route `StoryRoute num`))
  (`/Engine/EditorBlueprintResources/StandardMacros.IsValid` _output
    (:`Is Valid`
      (bind _location (`/Game/Rewind/Ai_Friendly/Bp_Story_Route.Get Spline Point as World Position` _output))
      (return _location _output))))

(fn `SetMovementSpeed`
  (params (Speed :type "/Game/Rewind/Ai_Enemy/AI/Enums/E_MovementSpeed Enum" :default "NewEnumerator0"))
  (returns (SpeedValue :type "Float (double-precision)"))
  (set `CharacterMovementComponent.MaxWalkSpeed` (select `/Game/Rewind/Ai_Enemy/AI/Enums/E_MovementSpeed` Speed :`NewEnumerator1` 100.0 :`NewEnumerator2` 300.0 :`NewEnumerator3` 500.0 :!type "Float (single-precision)") (`self.CharacterMovement`))
  (return 0.0))

(fn `UserConstructionScript`)
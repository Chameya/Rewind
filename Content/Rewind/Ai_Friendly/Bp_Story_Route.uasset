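; Story route actor for friendly AI that exposes the points of a StoryRoute spline as a sequence of world-space waypoints.
; IncrementStoryRoute steps the current index by Direction, while IcrementStory steps from a passed-in index; both set Direction to 1 at index zero.
; The last point triggers no reversal, and CheckIfFInished reports completion only when the index equals the point count.
; GetSplinePointAsWorldPosition returns the current waypoint's location.
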(event `IncrementStoryRoute`
  (bind _output_get (set `self.StoryRouteIndex` (+ (`self.StoryRouteIndex`) (`self.Direction`))))
  (if (== _output_get (- (`SplineComponent.GetNumberOfSplinePoints` (`self.StoryRoute`)) 1))
    _
    (elif (== (`self.StoryRouteIndex`) 0)
      (set `self.Direction` 1))))

(fn `Check If FInished`
  (returns (Output_Get :type Boolean))
  (if (== (`self.StoryRouteIndex`) (`SplineComponent.GetNumberOfSplinePoints` (`self.StoryRoute`)))
    (bind _output_get (set `self.Finished` true))
    (return _output_get)
    (else
      (bind _output_get_2 (set `self.Finished` false))
      (return _output_get_2))))

(fn `Get Spline Point as World Position`
  (returns (Location :type "Vector Structure"))
  (return (`SplineComponent.GetLocationAtSplinePoint` (`self.StoryRoute`) (`self.StoryRouteIndex`) "World")))

(fn `Icrement Story`
  (params (NewParam :type Integer))
  (bind _output_get (set `self.StoryRouteIndex` (+ NewParam (`self.Direction`))))
  (if (== _output_get (- (`SplineComponent.GetNumberOfSplinePoints` (`self.StoryRoute`)) 1))
    _
    (elif (== (`self.StoryRouteIndex`) 0)
      (set `self.Direction` 1))))

(fn `UserConstructionScript`)
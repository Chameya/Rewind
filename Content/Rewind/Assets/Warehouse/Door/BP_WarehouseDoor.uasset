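; Interactive warehouse door that the player opens and closes with the E key while standing near it.
; A box overlap with the third-person character enables input on the door for player 0, and leaving disables it.
; A FlipFlop alternates between playing a timeline and reversing it from the end, with the track driving the DoorFrame's relative yaw.
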(event `self.Box.OnComponentBeginOverlap`
  (params (OverlappedComponent :type "PrimitiveComponent Object Reference") (OtherActor :type "Actor Object Reference") (OtherComp :type "PrimitiveComponent Object Reference") (OtherBodyIndex :type Integer) (bFromSweep :type Boolean) (SweepResult :type "HitResult Structure (by ref)"))
  (cast `/Game/Rewind/VezamsMap/character/BP_ThirdPersonCharacterveezam` OtherActor)
  (`self.EnableInput` (`GameplayStatics.GetPlayerController` 0)))

(event `self.Box.OnComponentEndOverlap`
  (params (OverlappedComponent :type "PrimitiveComponent Object Reference") (OtherActor :type "Actor Object Reference") (OtherComp :type "PrimitiveComponent Object Reference") (OtherBodyIndex :type Integer))
  (cast `/Game/Rewind/VezamsMap/character/BP_ThirdPersonCharacterveezam` OtherActor)
  (`self.DisableInput` (`GameplayStatics.GetPlayerController` 0)))

(event `Key|E`
  (params (Key :type "Key Structure"))
  (:`Pressed`
    (`/Engine/EditorBlueprintResources/StandardMacros.FlipFlop`
      (:`A`
        (bind (_direction _newtrack_0) (`Timeline|DoorRotateTimeline` :!label _label)
          (:`Update`
            (`SceneComponent.K2_SetRelativeRotation` (`self.DoorFrame`) (`KismetMathLibrary.MakeRotator` 0.0 0.0 _newtrack_0) false false))))
      (:`B`
        (goto _label :!via `ReverseFromEnd`)))))

(fn `UserConstructionScript`)